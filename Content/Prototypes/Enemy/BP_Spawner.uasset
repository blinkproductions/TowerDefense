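; Enemy spawner prototype that endlessly spawns AI pawns at its Arrow component's location.
; On BeginPlay it caches the first TargetPoint in the level as TargetLocation, waits out a pre-start countdown, then starts a looping one-second timer.
; Each tick of that timer spawns the next EnemiesToSpawn class with the BT_Enemy behavior tree, using a modulo index to cycle the list.
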(event `self.ReceiveBeginPlay`
  (bind _outactors (`GameplayStatics.GetAllActorsOfClass` "/Script/Engine.TargetPoint"))
  (set `self.TargetLocation` (`|GetArrayItem` _outactors))
  (`KismetSystemLibrary.Delay` (`self.PreStartCountdown`))
  (`KismetSystemLibrary.K2_SetTimerDelegate` (delegate `SpawnEnemy`) 1.0 true))

(event `SpawnEnemy`
  (bind _enemiestospawn (`self.EnemiesToSpawn`))
  (bind _returnvalue_location (`KismetMathLibrary.BreakTransform` (`SceneComponent.K2_GetComponentToWorld` (`self.Arrow`))))
  (`AIBlueprintHelperLibrary.SpawnAIFromClass` (`|GetArrayItem` _enemiestospawn (mod (`self.Index`) (`KismetArrayLibrary.Array_Length` _enemiestospawn))) "/Game/Prototypes/Enemy/BT_Enemy.BT_Enemy" _returnvalue_location (struct) false null)
  (`/Engine/EditorBlueprintResources/StandardMacros.IncrementInt` (`self.Index`)))

(fn `UserConstructionScript`)