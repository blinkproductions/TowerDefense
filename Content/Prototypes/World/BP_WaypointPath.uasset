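; BP_WaypointPath is a prototype patrol path that exposes the points of a spline as waypoints.
; IncrementPatrolPath advances a wrapping PatrolIndex, and GetNextWaypointAsWorldPosition reads that point's world location straight from the spline.
; BeginPlay also caches local-space point transforms in a Waypoints array, which in this graph only feeds a debug print of every location on each Tick.
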(event `self.ReceiveBeginPlay`
  (`self.InitializeWaypoints`))

(event `self.ReceiveTick`
  (params (DeltaSeconds :type "Float (single-precision)"))
  (`self.DebugWaypoints`))

(event `IncrementPatrolPath`
  (set `self.PatrolIndex` (mod (+ (`self.PatrolIndex`) 1) (`SplineComponent.GetNumberOfSplinePoints` (`self.Spline`)))))

(fn `DebugWaypoints`
  (for (_array_element _array_index) (`self.Waypoints`)
    (`KismetSystemLibrary.PrintString` (`KismetTextLibrary.Conv_TextToString` (`|FormatText` "(BP_WayponitPath)Index {index}: Location: ({x},{y},{z})" _array_index (.x (.location _array_element)) (.y (.location _array_element)) (.z (.location _array_element)))) true true (struct :`G` 0.66 :`B` 1.0 :`A` 1.0) 0.0)))

(fn `GetNextWaypointAsWorldPosition`
  (returns (ReturnValue :type "Vector Structure"))
  (return (`SplineComponent.GetLocationAtSplinePoint` (`self.Spline`) (`self.PatrolIndex`) "World")))

(fn `InitializeWaypoints`
  (`KismetArrayLibrary.Array_Resize` (`self.Waypoints`) (`SplineComponent.GetNumberOfSplinePoints` (`self.Spline`)))
  (for _index (range (`KismetArrayLibrary.Array_Length` (`self.Waypoints`)))
    (`KismetArrayLibrary.Array_Set` (`self.Waypoints`) _index (`SplineComponent.GetTransformAtSplinePoint` (`self.Spline`) _index "Local" false))))

(fn `UserConstructionScript`)