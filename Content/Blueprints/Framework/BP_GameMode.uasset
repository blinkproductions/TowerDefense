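; Game mode for what appears to be a card-dealing tower defense game, running the card deck, wave-based tier unlocks and gold checks.
; After BeginPlay it deals three cards and grants starting gold, while a Delay on Tick throttles further deals, each refreshing the HUD conveyor belt.
; DetermineTiersUnlocked widens tiers and dealing range by wave, and VerifyGold checks affordability.
; Tick also prints deck, wave, tier and gold debug text.
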(event `self.ReceiveBeginPlay`
  (bind _asbp_camera_pawn (cast `/Game/Blueprints/Player/BP_CameraPawn` (`GameplayStatics.GetPlayerPawn` 0)))
  (set `self.PlayerRef` _asbp_camera_pawn)
  (bind _asbp_td_player_controller (cast `/Game/Blueprints/Player/BP_TD_PlayerController` (`GameplayStatics.GetPlayerController` 0)))
  (set `self.PlayerControllerRef` _asbp_td_player_controller)
  (`KismetSystemLibrary.Delay` 0.2)
  (`self.InitializeDeck`)
  (`self.GiveStartingGold` 50))

(event `self.ReceiveTick`
  (params (DeltaSeconds :type "Float (single-precision)"))
  (`|ExecutionSequence`
    (:`then_0`
      (`KismetSystemLibrary.Delay` (`self.DealingDelay`))
      (`self.DealCardToDealingPile`))
    (:`then_1`
      ;[1 1 1] Debug Prints
      (`self.DebugDealingDeck`))
    (:`then_2`
      (bind _returnvalue (`self.GetCurentGold`))
      (`KismetSystemLibrary.PrintString` (`KismetTextLibrary.Conv_TextToString` (`|FormatText` "(BP_GameMode)CurrentGold: {gold}" _returnvalue)) true true (struct :`G` 0.66 :`B` 1.0 :`A` 1.0) 0.0))))

(fn `DealCardToDealingPile`
  (`/Game/Prototypes/ActorComponents/DeckOfCards.DealACard` (`self.DeckOfCards`) self)
  (`self.UpdateDealingPile`))

(fn `DebugDealingDeck`
  (bind _cardtobeburned_name (break `UnitProperties` (`/Game/Prototypes/ActorComponents/DeckOfCards.CardToBeBurned` (`self.DeckOfCards`))))
  (`|ExecutionSequence`
    (:`then_0`
      ;[1 1 1] Debugging DeckOfCardsDealt
      (`KismetSystemLibrary.PrintString` (`KismetTextLibrary.Conv_TextToString` (`|FormatText` "(BP_GameMode)Card Burnt: {name}" _cardtobeburned_name)) true true (struct :`R` 1.0 :`G` 0.088168 :`A` 1.0) 0.0)
      (for (_array_element _array_index) (`/Game/Prototypes/ActorComponents/DeckOfCards.DeckOfCards` (`self.DeckOfCards`))
        (bind (_name _unittype _thumbnail _attacktype _unitclass _tier) (break `UnitProperties` _array_element))
        (`KismetSystemLibrary.PrintString` (`KismetTextLibrary.Conv_TextToString` (`|FormatText` "(BP_GameMode)Card {Index}: \n   Tier: {Tier} \n   UnitName: {Name}" (+ _array_index 1) _tier _name)) true true (struct :`R` 0.348958 :`G` 0.323141 :`A` 1.0) 0.0)))
    (:`then_1`
      ;[1 1 1] Print CurrentWave inside GameMode
      (`KismetSystemLibrary.PrintString` (`KismetTextLibrary.Conv_TextToString` (`|FormatText` "(BP_GameMode)CurrentWave: {wave}" (`self.CurrentWave`))) true true (struct :`R` 0.099663 :`G` 1.0 :`A` 1.0) 0.0))
    (:`then_2`
      ;[1 1 1] Print status of Tiers
      (for (_array_element_2 _array_index_2) (`self.TiersUnlocked`)
        (`KismetSystemLibrary.PrintString` (`KismetTextLibrary.Conv_TextToString` (`|FormatText` "(BP_GameMode)Tier {Tier}: {unlocked}" (+ _array_index_2 1) _array_element_2)) true true (struct :`R` 1.0 :`G` 0.005552 :`A` 1.0) 0.0)))))

(fn `DetermineTiersUnlocked`
  (bind _currentwave (`self.CurrentWave`))
  ;[1 1 1] Tier 1 and 2 unlocked
  (if (and (> _currentwave 5) (<= _currentwave 10))
    (`KismetArrayLibrary.Array_Set` (`self.TiersUnlocked`) (- 2 1) true)
    (set `self.DealingRange` 16)
    (else
      ;[1 1 1] All Tiers unlocked
      (if (> (`self.CurrentWave`) 10)
        (for (_ _array_index) (`self.TiersUnlocked`)
          (`KismetArrayLibrary.Array_Set` (`self.TiersUnlocked`) _array_index true)
          (set `self.DealingRange` 25))))))

(fn `InitializeDeck`
  (bind _deckofcards (`self.DeckOfCards`))
  (`/Game/Prototypes/ActorComponents/DeckOfCards.DealACard` _deckofcards self)
  (`/Game/Prototypes/ActorComponents/DeckOfCards.DealACard` _deckofcards self)
  (`/Game/Prototypes/ActorComponents/DeckOfCards.DealACard` _deckofcards self)
  (`self.UpdateDealingPile`))

(fn `UpdateDealingPile`
  (`/Game/UserInterface/Widgets/CardRelatedWidgets/WBP_ConveyorBelt.UpdateWidget` (`/Game/UserInterface/Widgets/WBP_HUD.WBP_ConveyorBelt` (`/Game/Blueprints/Player/BP_TD_PlayerController.HUDRef` (`self.PlayerControllerRef`)))))

(fn `UserConstructionScript`)

(fn `VerifyGold`
  (params (PriceToPay :type Integer))
  (returns (bCanBuy :type Boolean))
  (bind _returnvalue (`self.GetCurentGold`))
  (if (>= _returnvalue PriceToPay)
    (return true)
    (else
      (return false))))