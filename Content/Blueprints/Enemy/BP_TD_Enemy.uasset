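; Base tower defense enemy that shows health and armor on a widget bar and rewards gold when killed.
; BeginPlay caches the bar widget and sets its max health from the HealthComponent, and UpdateHealth refreshes health and armor percentages plus a clamped current health value.
; Tick polls the component's IsDead flag, then spawns an explosion, gives GoldReward through BP_GameMode and destroys the actor.
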(event `self.ReceiveBeginPlay`
  ;[1 1 1] Initialize ArmorAndHealthBar widget
  (bind _aswbp_armor_and_health_bar (cast `/Game/UserInterface/Widgets/WBP_ArmorAndHealthBar` (`WidgetComponent.GetUserWidgetObject` (`self.ArmorAndHealthWidget`))))
  (bind _output_get (set `self.ArmorAndHealthWidgetRef` _aswbp_armor_and_health_bar))
  (set `/Game/UserInterface/Widgets/WBP_ArmorAndHealthBar.MaxHealth` (`KismetMathLibrary.FTrunc` (`HealthComponent.MaxHealth` (`self.HealthComponent`))) _output_get))

(event `self.ReceiveTick`
  (params (DeltaSeconds :type "Float (single-precision)"))
  (if (`HealthComponent.bIsDead` (`self.HealthComponent`))
    (`GameplayStatics.SpawnEmitterAtLocation` "/Game/StarterContent/Particles/P_Explosion.P_Explosion" (`self.K2_GetActorLocation`))
    (bind _asbp_game_mode (cast `/Game/Blueprints/Framework/BP_GameMode` (`GameplayStatics.GetGameMode`)))
    (`TowerDefenseGameModeBase.GiveGold` _asbp_game_mode (`self.GoldReward`))
    (`self.K2_DestroyActor`)))

(event `self.UpdateHealth`
  (bind _armorandhealthwidgetref (`self.ArmorAndHealthWidgetRef`))
  (bind _healthcomponent (`self.HealthComponent`))
  ;[1 1 1] Health Manager
  (set `ArmorAndHealthBarWidget.HealthAmount` (`HealthComponent.GetCurrentHealthPercentage` _healthcomponent) _armorandhealthwidgetref)
  (set `ArmorAndHealthBarWidget.ArmorAmount` (`HealthComponent.GetCurrentArmorPercentage` _healthcomponent) _armorandhealthwidgetref)
  (set `/Game/UserInterface/Widgets/WBP_ArmorAndHealthBar.CurrentHealth` (`KismetMathLibrary.Clamp` (`KismetMathLibrary.FTrunc` (`HealthComponent.CurrentHealth` (`self.HealthComponent`))) 0 (`KismetMathLibrary.FTrunc` (`HealthComponent.MaxHealth` (`self.HealthComponent`)))) _armorandhealthwidgetref))

(fn `UserConstructionScript`)