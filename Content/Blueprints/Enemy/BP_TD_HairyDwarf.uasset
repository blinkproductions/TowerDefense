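; BP_TD_HairyDwarf is an enemy Blueprint, apparently for a tower defense game, that shows its health and armor on a widget bar.
; BeginPlay casts the ArmorAndHealthWidget component's user widget to WBP_ArmorAndHealthBar and caches the reference.
; UpdateHealth copies current health and armor percentages from HealthComponent into that widget, so the bar updates on that event rather than on Tick.
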(event `self.ReceiveBeginPlay`
  (bind _aswbp_armor_and_health_bar (cast `/Game/UserInterface/WBP_ArmorAndHealthBar` (`WidgetComponent.GetUserWidgetObject` (`self.ArmorAndHealthWidget`))))
  (set `self.ArmorAndHealthWidgetRef` _aswbp_armor_and_health_bar))

(event `self.UpdateHealth`
  (bind _armorandhealthwidgetref (`self.ArmorAndHealthWidgetRef`))
  (bind _healthcomponent (`self.HealthComponent`))
  (set `ArmorAndHealthBarWidget.HealthAmount` (`HealthComponent.GetCurrentHealthPercentage` _healthcomponent) _armorandhealthwidgetref)
  (set `ArmorAndHealthBarWidget.ArmorAmount` (`HealthComponent.GetCurrentArmorPercentage` _healthcomponent) _armorandhealthwidgetref))

(fn `UserConstructionScript`)